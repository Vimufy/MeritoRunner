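; Magnet power-up pickup for the runner game that sets the runner character's IsMagnetActive flag for a few seconds when touched.
; On overlap it plays a coin sound and hides itself, then, if the magnet was inactive, waits out a delay, clears the flag and destroys itself.
; If the magnet is already active it only stays hidden, and overlapping an obstacle wall destroys it.
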(event Collision|EventActorBeginOverlap
  (params (OtherActor :type Actor%20Object%20Reference))
  (Utilities|FlowControl|Sequence
    (:then_0
      (bind _asbp_runner_character (Utilities|Casting|CastToBP_RunnerCharacter OtherActor))
      (Utilities|Casting|CastToBP_RunnerGameMode (Game|GetGameMode))
      (Audio|PlaySound2D "/Game/Runner/Meshes/350874__cabled_mess__coin_c_08.350874__cabled_mess__coin_c_08" 1.0 1.0 0.0 0 0)
      (Rendering|SetActorHiddenInGame true)
      (if (not (Variables|/Game/Runner/Blueprints/BP_RunnerCharacter.BP_RunnerCharacter_C|GetIs%20Magnet%20Active? _asbp_runner_character))
        (Variables|/Game/Runner/Blueprints/BP_RunnerCharacter.BP_RunnerCharacter_C|SetIs%20Magnet%20Active? _asbp_runner_character true)
        (Development|PrintString "Magnet Active")
        (Utilities|FlowControl|Delay 5.0)
        (bind _asbp_runner_character_2 (Utilities|Casting|CastToBP_RunnerCharacter (Game|GetPlayerCharacter 0)))
        (Variables|/Game/Runner/Blueprints/BP_RunnerCharacter.BP_RunnerCharacter_C|SetIs%20Magnet%20Active? _asbp_runner_character_2 false)
        (Development|PrintString "Magnet Inactive")
        (Actor|DestroyActor)))
    (:then_1
      (Utilities|Casting|CastToBP_Obstacles_Wall OtherActor)
      (Actor|DestroyActor))))

(fn ConstructionScript)