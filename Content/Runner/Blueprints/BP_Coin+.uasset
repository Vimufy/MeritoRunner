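; Coin pickup for a runner game that adds to the game mode's coin count, plays a sound and updates the runner character's coins.
; The coin also destroys itself when it overlaps a wall obstacle or magnet power-up.
; A separate Sphere overlap checks whether the runner's magnet is active, then starts a timeline that pulls the coin toward the player using VInterpTo plus a timeline offset.
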(event OnComponentBeginOverlap(Sphere)
  (params (OverlappedComponent :type Primitive%20Component%20Object%20Reference) (OtherActor :type Actor%20Object%20Reference) (OtherComp :type Primitive%20Component%20Object%20Reference) (OtherBodyIndex :type Integer) (bFromSweep :type Boolean) (SweepResult :type Hit%20Result%20Structure%20%28by%20ref%29))
  (bind _asbp_runner_character (Utilities|Casting|CastToBP_RunnerCharacter OtherActor))
  (if (Variables|/Game/Runner/Blueprints/BP_RunnerCharacter.BP_RunnerCharacter_C|GetIs%20Magnet%20Active? _asbp_runner_character)
    (bind _transition (Timeline|Oś%20czasu PlayFromStart)
      (:Update
        (Transformation|SetActorLocation (+ _transition (Math|Interpolation|VInterpTo (.Location (Math|Transform|BreakTransform (Transformation|GetActorTransform))) (Transformation|GetActorLocation (Game|GetPlayerCharacter 0)) (Utilities|Time|GetWorldDeltaSeconds) 2e+01)) false false)))))

(event OnComponentBeginOverlap(Coin)
  (params (OverlappedComponent :type Primitive%20Component%20Object%20Reference) (OtherActor :type Actor%20Object%20Reference) (OtherComp :type Primitive%20Component%20Object%20Reference) (OtherBodyIndex :type Integer) (bFromSweep :type Boolean) (SweepResult :type Hit%20Result%20Structure%20%28by%20ref%29))
  (Utilities|FlowControl|Sequence
    (:then_0
      (bind _asbp_runner_character (Utilities|Casting|CastToBP_RunnerCharacter OtherActor))
      (bind _asbp_runner_game_mode (Utilities|Casting|CastToBP_RunnerGameMode (Game|GetGameMode)))
      (bind _result (Math|Integer|IncrementInt (Variables|/Game/Runner/Blueprints/BP_RunnerGameMode.BP_RunnerGameMode_C|GetCoins _asbp_runner_game_mode))
        (:%20%20
          (Development|PrintString (Utilities|String|ToString(Integer) _result) true false "(R=0.977702,G=1.000000,B=0.200223,A=1.000000)")
          (Audio|PlaySound2D "/Game/Runner/Meshes/350874__cabled_mess__coin_c_08.350874__cabled_mess__coin_c_08" 1.0 1.0 0.0 0 0)
          (Actor|DestroyActor)
          (Default|UpdateCoins _asbp_runner_character))))
    (:then_1
      (Utilities|Casting|CastToBP_Obstacles_Wall OtherActor)
      (Actor|DestroyActor))
    (:then_2
      (Utilities|Casting|CastToBP_PowerUP_Magnet+ OtherActor)
      (Actor|DestroyActor))))

(fn ConstructionScript)